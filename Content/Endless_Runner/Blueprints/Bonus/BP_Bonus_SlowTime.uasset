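; Endless-runner bonus pickup that briefly slows time for the whole game.
; When a RunnerCharacter overlaps its StaticMesh, it plays a shout, hides the Scene component without propagating to children, and halves global time dilation.
; After a Delay it restores normal speed and destroys itself.
; The Delay runs in dilated time, so the slowdown lasts about four real seconds, not the five its comment states.
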(event `self.StaticMesh.OnComponentBeginOverlap`
  (params (OverlappedComponent :type "PrimitiveComponent Object Reference") (OtherActor :type "Actor Object Reference") (OtherComp :type "PrimitiveComponent Object Reference") (OtherBodyIndex :type Integer) (bFromSweep :type Boolean) (SweepResult :type "HitResult Structure (by ref)"))
  ;[1 1 1] Замедление времени всего на 5 сек
  (cast `/Game/Endless_Runner/Blueprints/Character/RunnerCharacter` OtherActor)
  (`GameplayStatics.PlaySoundAtLocation` "/Game/HumanVocalizations/HumanMaleB/Wavs/voice_male_b_battle_shout_short_03.voice_male_b_battle_shout_short_03" (`self.K2_GetActorLocation`) (struct) 1.0 1.0 0.0 null null null)
  (`SceneComponent.SetVisibility` (`self.Scene`) false false)
  (`KismetSystemLibrary.PrintString` "5")
  (`GameplayStatics.SetGlobalTimeDilation` 0.5)
  (`KismetSystemLibrary.Delay` 2.0)
  (`KismetSystemLibrary.PrintString` "end")
  (`GameplayStatics.SetGlobalTimeDilation` 1.0)
  (`self.K2_DestroyActor`))

(fn `UserConstructionScript`)