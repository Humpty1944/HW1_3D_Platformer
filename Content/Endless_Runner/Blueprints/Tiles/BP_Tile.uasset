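; Floor tile for the endless runner that randomly populates itself with coins and either an arrow or a possible blocker, wall-walk or slow-time item.
; The construction script places these as child actors at spawn points and coin areas.
; End trigger counts passed tiles; every tenth starts a level, adjusts its own odds, adds tiles, speeds the runner and destroys itself.
; JumpEnd kills fallen players, and Tick toggles wall collision while wall-walk is active.
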(event `self.ReceiveTick`
  (params (DeltaSeconds :type "Float (single-precision)"))
  ;[1 1 1] Каждый тик проверяем, дейсвтует ли проход через стены. Если да, то позволяем игроку проходить сквозь них, иначе запрет
  (bind _asrunner_character (cast `/Game/Endless_Runner/Blueprints/Character/RunnerCharacter` (`GameplayStatics.GetPlayerCharacter` 0)))
  (if (`/Game/Endless_Runner/Blueprints/Character/RunnerCharacter.isWalkActive` _asrunner_character)
    (`PrimitiveComponent.SetCollisionResponseToAllChannels` (`self.Wall2`) "ECR_Overlap")
    (`PrimitiveComponent.SetCollisionResponseToAllChannels` (`self.Wall3`) "ECR_Overlap")
    (else
      (`PrimitiveComponent.SetCollisionResponseToAllChannels` (`self.Wall2`) "ECR_Block")
      (`PrimitiveComponent.SetCollisionResponseToAllChannels` (`self.Wall3`) "ECR_Block"))))

(event `self.EndTrigger.OnComponentBeginOverlap`
  (params (OverlappedComponent :type "PrimitiveComponent Object Reference") (OtherActor :type "Actor Object Reference") (OtherComp :type "PrimitiveComponent Object Reference") (OtherBodyIndex :type Integer) (bFromSweep :type Boolean) (SweepResult :type "HitResult Structure (by ref)"))
  ;[1 1 1] Игрок прошел плитку, происходит генерация следующих, если прошел 10 плиток (уровень)
  (bind _asrunner_character (cast `/Game/Endless_Runner/Blueprints/Character/RunnerCharacter` OtherActor))
  (bind _asrunner_game_mode (cast `/Game/Endless_Runner/GameMode/RunnerGameMode` (`GameplayStatics.GetGameMode`)))
  (bind _output_get (set `/Game/Endless_Runner/GameMode/RunnerGameMode.PassTile` (+ (`/Game/Endless_Runner/GameMode/RunnerGameMode.PassTile` _asrunner_game_mode) 1) _asrunner_game_mode))
  (if (== (mod _output_get 10) 0)
    (`self.ChangePossibility`)
    (`/Game/Endless_Runner/GameMode/RunnerGameMode.New Level` _asrunner_game_mode)
    (for _ (range 11)
      (`/Game/Endless_Runner/GameMode/RunnerGameMode.AddFloorTile` _asrunner_game_mode))
    (bind _charactermovement (`Character.CharacterMovement` _asrunner_character))
    (set `CharacterMovementComponent.MaxWalkSpeed` (`KismetMathLibrary.FClamp` (* (`MovementComponent.GetMaxSpeed` _charactermovement) 1.03) 0.0 2000.0) _charactermovement)
    (`KismetSystemLibrary.Delay` 2.0)
    (`self.K2_DestroyActor`)))

(event `self.JumpEnd.OnComponentBeginOverlap`
  (params (OverlappedComponent :type "PrimitiveComponent Object Reference") (OtherActor :type "Actor Object Reference") (OtherComp :type "PrimitiveComponent Object Reference") (OtherBodyIndex :type Integer) (bFromSweep :type Boolean) (SweepResult :type "HitResult Structure (by ref)"))
  ;[1 1 1] If player fell into abyss, box collision occurs
  (bind _asrunner_character (cast `/Game/Endless_Runner/Blueprints/Character/RunnerCharacter` OtherActor))
  (`/Game/Endless_Runner/Blueprints/Character/RunnerCharacter.Death` _asrunner_character))

(event `self.JumpEnd.OnComponentHit`
  (params (HitComponent :type "PrimitiveComponent Object Reference") (OtherActor :type "Actor Object Reference") (OtherComp :type "PrimitiveComponent Object Reference") (NormalImpulse :type "Vector Structure") (Hit :type "HitResult Structure (by ref)")))

(fn `ChangePossibility`
  ;[1 1 1] С каждым новым уровнем меняем вероятности появления различных предметов
  (set `self.PossibiltyOfNothing` (`KismetMathLibrary.FClamp` (- (`self.PossibiltyOfNothing`) 0.05) 0.05)))

(fn `Get Attach Transform`
  (returns (`Attach Transform` :type "Transform Structure"))
  (return (`SceneComponent.K2_GetComponentToWorld` (`self.AttachPoint`))))

(fn `SetSpawnPoint`
  (set `self.SpawnPoints` (`|MakeArray` (`SceneComponent.GetRelativeTransform` (`self.SpawnPoint`)) (`SceneComponent.GetRelativeTransform` (`self.SpawnPointR`)) (`SceneComponent.GetRelativeTransform` (`self.SpawnPointL`)))))

(fn `Spawn Walk Wall`
  (bind _spawnpoints (`self.SpawnPoints`))
  (`AddComponent|NODE_AddChildActorComponent-8` :`RelativeTransform` (`|GetArrayItem` _spawnpoints (`KismetMathLibrary.RandomIntegerInRange` 0 (`KismetArrayLibrary.Array_LastIndex` _spawnpoints)))))

(fn `SpawnArrow`
  (`AddComponent|NODE_AddChildActorComponent-7` :`RelativeTransform` (`KismetMathLibrary.Conv_VectorToTransform` (`SceneComponent.RelativeLocation` (`self.ArrowArrow`)))))

(fn `SpawnBlocker`
  (bind _spawnpoints (`self.SpawnPoints`))
  (`AddComponent|NODE_AddChildActorComponent-0` :`RelativeTransform` (`|GetArrayItem` _spawnpoints (`KismetMathLibrary.RandomIntegerInRange` 0 (`KismetArrayLibrary.Array_LastIndex` _spawnpoints)))))

(fn `SpawnCoins`
  (bind _returnvalue (`KismetMathLibrary.RandomFloatInRange` 0.0 1.0))
  (bind _coin_area3 (`self.Coin Area3`))
  (bind _coin_area1 (`self.Coin Area1`))
  (bind _coin_area2 (`self.Coin Area2`))
  (if (`KismetMathLibrary.InRange_FloatFloat` _returnvalue 0.0 0.3)
    (for _ (range 3)
      (`AddComponent|NODE_AddChildActorComponent-10` :`RelativeTransform` (`KismetMathLibrary.Conv_VectorToTransform` (`KismetMathLibrary.RandomPointInBoundingBox` (`SceneComponent.RelativeLocation` _coin_area1) (`BoxComponent.BoxExtent` _coin_area1)))))
    (elif (`KismetMathLibrary.InRange_FloatFloat` _returnvalue 0.3 0.6)
      (for _ (range 3)
        (`AddComponent|NODE_AddChildActorComponent-11` :`RelativeTransform` (`KismetMathLibrary.Conv_VectorToTransform` (`KismetMathLibrary.RandomPointInBoundingBox` (`SceneComponent.RelativeLocation` _coin_area2) (`BoxComponent.BoxExtent` _coin_area2)))))
      (else
        (for _ (range 3)
          (`AddComponent|NODE_AddChildActorComponent-12` :`RelativeTransform` (`KismetMathLibrary.Conv_VectorToTransform` (`KismetMathLibrary.RandomPointInBoundingBox` (`SceneComponent.RelativeLocation` _coin_area3) (`BoxComponent.BoxExtent` _coin_area3)))))))))

(fn `SpawnSlowTime`
  (bind _spawnpoints (`self.SpawnPoints`))
  (`AddComponent|NODE_AddChildActorComponent-9` :`RelativeTransform` (`|GetArrayItem` _spawnpoints (`KismetMathLibrary.RandomIntegerInRange` 0 (`KismetArrayLibrary.Array_LastIndex` _spawnpoints)))))

(fn `UserConstructionScript`
  ;[1 1 1] Генерим каждый объект с заданной вероятностью (перемнные с названиями "Possibility...")
  (set `self.PossibilityDuringThisTile` (`KismetMathLibrary.RandomFloatInRange` 0.0 1.0))
  (`self.SetSpawnPoint`)
  (if (<= (`KismetMathLibrary.RandomFloatInRange` 0.0 1.0) 0.5)
    (`self.SpawnCoins`))
  (if (<= (`self.PossibilityDuringThisTile`) (`self.PossibiltyOfNothing`))
    (switch `int` (`KismetMathLibrary.RandomIntegerInRange` 0 2)
      (:`0`
        (`self.SpawnBlocker`))
      (:`1`
        (if (<= (`KismetMathLibrary.RandomFloatInRange` 0.0 1.0) 0.55)
          (switch `int` (`KismetMathLibrary.RandomIntegerInRange` 0 1)
            (:`Default`
              (`self.Spawn Walk Wall`))
            (:`0`
              (`self.SpawnSlowTime`))))))
    (else
      (`self.SpawnArrow`))))